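; Dash ability Blueprint that moves an assigned character horizontally along its forward vector, using limited charges.
; CallDash spends a charge and runs a looping per-frame timer calling LaunchCharacter until DashDuration ends, leaving SpeedIntensity unused.
; The assigned collider generates overlap events during the dash and stops afterward.
; Tick refills charges one at a time on a cooldown, which restarts with each dash.
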(event Custom|CallDash
  (params (SpeedIntensity :type Float%20%28single-precision%29))
  (if (not (Variables|Default|GetIsDashing))
    (if (> (Variables|Default|GetDashReload) 0)
      (Utilities|FlowControl|Sequence
        (:then_0
          (Variables|/Script/Engine.PrimitiveComponent|SetbGenerateOverlapEvents (Variables|Default|GetCollider) true)
          (bind _returnvalue (Utilities|Time|SetTimerbyFunctionName 0 "DashForward" (Utilities|Time|GetWorldDeltaSeconds) true))
          (CallFunction|AddDashLoad -1)
          (Variables|Default|SetCurrentCoolDownDashLoad (Variables|Default|GetCooldownDashLoad)))
        (:then_1
          (Utilities|FlowControl|Delay (Variables|Default|GetDashDuration))
          (Utilities|Time|PauseTimerbyHandle _returnvalue)
          (Variables|Default|SetIsDashing false)
          (Variables|/Script/Engine.PrimitiveComponent|SetbGenerateOverlapEvents (Variables|Default|GetCollider) false))))))

(event EventBeginPlay
  (Variables|Default|SetDashReload (Variables|Default|GetMaxDashReload)))

(event EventTick
  (params (DeltaSeconds :type Float%20%28single-precision%29))
  (if (< (Variables|Default|GetDashReload) (Variables|Default|GetMaxDashReload))
    (CallFunction|CoolDownDashTimer)))

(fn DashForward
  (bind _dashspeed (Variables|Default|GetDashSpeed))
  (bind _entity (Variables|Default|GetEntity))
  (bind _returnvalue (Transformation|GetActorForwardVector _entity))
  (bind _returnvalue_2 (* _returnvalue _dashspeed))
  (bind (_x _y) (Math|Vector|BreakVector _returnvalue_2))
  (Variables|Default|SetIsDashing true)
  (bind _ascharacter (Utilities|Casting|CastToCharacter (Variables|Default|GetEntity))
    (:then
      (Character|LaunchCharacter _ascharacter (Math|Vector|MakeVector _x _y 0.0) true false))
    (:CastFailed
      (Development|PrintString "Entity have no character component"))))

(fn SetEntity
  (params (Entity :type Character%20Object%20Reference))
  (Variables|Default|SetEntity Entity))

(fn SetIsDashing
  (params (Value :type Boolean))
  (Variables|Default|SetIsDashing Value))

(fn SetCapsuleCollider
  (params (Collider :type Capsule%20Component%20Object%20Reference))
  (Variables|Default|SetCollider Collider))

(fn AddDashLoad
  (params (Value :type Integer))
  (Variables|Default|SetDashReload (Math|Integer|Clamp(Integer) (+ (Variables|Default|GetDashReload) Value) 0 (Variables|Default|GetMaxDashReload))))

(fn CheckDashLoad
  (if (>= (Variables|Default|GetDashReload) (Variables|Default|GetMaxDashReload))
    (Variables|Default|SetCurrentCoolDownDashLoad 0.0)
    (else
      (Variables|Default|SetCurrentCoolDownDashLoad (Variables|Default|GetCooldownDashLoad)))))

(fn CoolDownDashTimer
  (if (> (Variables|Default|GetCurrentCoolDownDashLoad) 0.0)
    (Variables|Default|SetCurrentCoolDownDashLoad (- (Variables|Default|GetCurrentCoolDownDashLoad) (Utilities|Time|GetWorldDeltaSeconds)))
    (else
      (Variables|Default|SetDashReload (+ (Variables|Default|GetDashReload) 1))
      (CallFunction|CheckDashLoad))))